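; Game mode Blueprint for Toon Tanks that creates the game's UI: main HUD, start screen and game over screen.
; BeginPlay adds the main widget and fills its tower count label from MTowersCount, and UpdateLeftTowerCount re-runs that same text update.
; StartGame and GameOver events add their widgets to the viewport, with the latter showing a win or loss message based on WonGame.
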(event EventBeginPlay
  (bind _returnvalue (UserInterface|CreateWidget "/Game/Blueprints/Widget/WBP_MainGameWidget.WBP_MainGameWidget_C"))
  (UserInterface|Viewport|AddtoViewport _returnvalue 0)
  (Rendering|Components|TextRender|SetText (Variables|/Game/Blueprints/Widget/WBP_MainGameWidget.WBP_MainGameWidget_C|GetLeftTowers _returnvalue) (Utilities|Text|ToText(String) (Utilities|String|Append "Left Tower Count : " (Utilities|String|ToString(Integer) (Variables|Default|GetmTowersCount))))))

(event EventStartGame
  (bind _returnvalue (UserInterface|CreateWidget "/Game/Blueprints/Widget/WBP_StartGameWidget.WBP_StartGameWidget_C"))
  (UserInterface|Viewport|AddtoViewport _returnvalue 0))

(event EventGameOver
  (params (bWonGame :type Boolean))
  (bind _returnvalue (UserInterface|CreateWidget "/Game/Blueprints/Widget/WBP_GameOverWidget.WBP_GameOverWidget_C"))
  (Rendering|Components|TextRender|SetText (Variables|/Game/Blueprints/Widget/WBP_GameOverWidget.WBP_GameOverWidget_C|GetDisplayText _returnvalue) (select bWonGame "You Win!" "You Lost"))
  (UserInterface|Viewport|AddtoViewport _returnvalue 0))

(event EventUpdateLeftTowerCount
  (Rendering|Components|TextRender|SetText (Variables|/Game/Blueprints/Widget/WBP_MainGameWidget.WBP_MainGameWidget_C|GetLeftTowers (stale EventBeginPlay _returnvalue)) (Utilities|Text|ToText(String) (Utilities|String|Append "Left Tower Count : " (Utilities|String|ToString(Integer) (Variables|Default|GetmTowersCount))))))

(fn ConstructionScript)